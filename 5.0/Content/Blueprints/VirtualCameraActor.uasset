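; A Cine Camera actor that works as a VR virtual camera, driven by a SteamVR tracked device such as a headset, remote or phone running iVRy.
; While TrackMotion is on, Tick reads the pose of the DeviceID device, adds position and per-axis rotation offsets, and writes it as the relative transform of the scene and camera components.
; Without room-scale tracking, only rotation follows the device.
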(event EventTick
  (params (DeltaSeconds :type Float%20%28single-precision%29))
  (bind _deviceid (Variables|Default|GetDeviceID))
  (bind (_outposition _outorientation) (Class|SteamVRFunctionLibrary|GetTrackedDevicePositionandOrientation _deviceid))
  (bind (_roll _pitch _yaw) (Math|Rotator|BreakRotator _outorientation))
  ;[1 1 1] VR Virtual Camera Link - This Cine Camera has been modified to accept input from a SteamVR tracked device. Headset is most likely 0, and the remotes are most likely 1 and 2. If you do not have a VR device, you can install iVRy on your phone and PC to use your smartphone as a SteamVR headset. If you have full-room VR setup, this will track both your camera's movement and rotation. Otherwise, the camera will be treated as stationary, and you can only track rotation.
  (if (Variables|Default|GetTrackMotion?)
    (Transformation|SetRelativeTransform (Variables|Default|GetSceneComponent) (Math|Transform|MakeTransform (+ _outposition (Variables|Default|GetPositionMod)) (Math|Rotator|MakeRotator (+ _roll (Variables|Default|GetXRollMod)) (+ _pitch (Variables|Default|GetYPitchMod)) (+ _yaw (Variables|Default|GetZYawMod))) "1,1,1") false false)))

(fn ConstructionScript)